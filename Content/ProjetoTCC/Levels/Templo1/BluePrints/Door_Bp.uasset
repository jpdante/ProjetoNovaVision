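; Openable door for the Templo1 level that can require a specific item from the player's inventory.
; Box overlap registers it as SymonCharacter's actionable actor and shows prompt texts; releasing F nearby checks the item and opens it.
; Repeated failed tries play a sound, with a BeginPlay Delay loop periodically clearing the counter.
; RotateOpen re-calls itself through short Delays, stepping yaw down to a fixed world angle; it never closes.
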(event OnComponentBeginOverlap(Box)
  (params (OverlappedComponent :type Primitive%20Component%20Object%20Reference) (OtherActor :type Actor%20Object%20Reference) (OtherComp :type Primitive%20Component%20Object%20Reference) (OtherBodyIndex :type Integer) (bFromSweep :type Boolean) (SweepResult :type Hit%20Result%20Structure%20%28by%20ref%29))
  (bind _assymon_character (Utilities|Casting|CastToSymonCharacter OtherActor))
  (Variables|/Game/ProjetoTCC/Characters/Main/SymonCharacter.SymonCharacter_C|SetActionableActorReference _assymon_character self)
  (Rendering|SetVisibility (Variables|Default|GetTextRender) true false)
  (Rendering|SetVisibility (Variables|Default|GetTextRender1) true false)
  (Variables|Default|SetPlayerIsClose true))

(event OnComponentEndOverlap(Box)
  (params (OverlappedComponent :type Primitive%20Component%20Object%20Reference) (OtherActor :type Actor%20Object%20Reference) (OtherComp :type Primitive%20Component%20Object%20Reference) (OtherBodyIndex :type Integer))
  (bind _assymon_character (Utilities|Casting|CastToSymonCharacter OtherActor))
  (Variables|/Game/ProjetoTCC/Characters/Main/SymonCharacter.SymonCharacter_C|SetActionableActorReference _assymon_character 0)
  (Rendering|SetVisibility (Variables|Default|GetTextRender) false false)
  (Rendering|SetVisibility (Variables|Default|GetTextRender1) false false)
  (Variables|Default|SetPlayerIsClose false))

(event Custom|RotateOpen
  (bind _returnvalue (Transformation|GetActorRotation))
  (bind (_roll _pitch _yaw) (Math|Rotator|BreakRotator _returnvalue))
  (if (<= _yaw -8e+01)
    (Variables|Default|SetDoorIsClosed false)
    (else
      (Transformation|SetActorRotation self (Math|Rotator|MakeRotator _roll _pitch (- _yaw 2.0)))
      (Utilities|FlowControl|Delay 0.01)
      (CallFunction|RotateOpen))))

(event EventBeginPlay
  (Utilities|FlowControl|Delay 5.0 :!label _label)
  (Variables|Default|SetTries 0)
  (Utilities|FlowControl|Delay 5.0)
  (goto _label))

(event Collision|EventActorBeginOverlap
  (params (OtherActor :type Actor%20Object%20Reference)))

(event EventTick
  (params (DeltaSeconds :type Float%20%28single-precision%29)))

(event EventFReleased
  (if (Variables|Default|GetPlayerIsClose)
    (if (Variables|Default|GetDoorIsClosed)
      (if (Variables|Default|GetNeedItem)
        (Utilities|IsValid (stale OnComponentBeginOverlap(Box) _assymon_character)
          (:Is%20Valid
            (if (Utilities|Array|ContainsItem (Variables|/Game/ProjetoTCC/Characters/Main/SymonCharacter.SymonCharacter_C|GetInventoryItems (stale OnComponentBeginOverlap(Box) _assymon_character)) (Variables|Default|GetItemType))
              (CallFunction|RotateOpen :!label _label)
              (else
                (bind _output_get (Variables|Default|SetTries (+ (Variables|Default|GetTries) 1)))
                (if (>= _output_get 5)
                  (Audio|PlaySound2D "/Game/ProjetoTCC/Levels/Templo1/BluePrints/Sounds/zua1.zua1")
                  (Variables|Default|SetTries 0))))))
        (else
          (goto _label))))))

(fn ConstructionScript)