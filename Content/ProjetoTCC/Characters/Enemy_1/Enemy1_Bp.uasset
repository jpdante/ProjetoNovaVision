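; Enemy character that patrols waypoints, chases the player and attacks with a sword spawned onto its weapon socket.
; A self-calling AI MoveTo loop cycles the waypoints with a delay between moves.
; PawnSensing starts a chase of SymonCharacter, then messages the AnimInstance to attack when close and allowed.
; Events gate attacks, set the sword's attacking flag and apply damage, either moving toward the attacker or ragdolling before destruction.
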(event OnSeePawn(PawnSensing)
  (params (Pawn :type Pawn%20Object%20Reference))
  (bind _self self)
  ;[1 1 1] Comment
  (bind _assymon_character (Utilities|Casting|CastToSymonCharacter Pawn))
  (AI|AIMoveTo _self "0, 0, 0" _assymon_character 8e+01 true
    (:then
      (Variables|/Script/Engine.CharacterMovementComponent|SetMaxWalkSpeed (Variables|Character|GetCharacterMovement) 2.7e+02))
    (:OnSuccess
      (if (<= (Transformation|GetDistanceTo _assymon_character _self) 3e+02)
        (Transformation|SetActorRotation _self (Math|Rotator|FindLookatRotation (Transformation|GetActorLocation _self) (Transformation|GetActorLocation _assymon_character)))
        (if (Variables|Default|GetAllowAttacking)
          (Class|Enemy1MoveInterface|AttackBl(Message) (Components|SkeletalMesh|GetAnimInstance (Variables|Character|GetMesh))))))))

(event Custom|ReduceHealth
  (params (Quantity :type Float%20%28single-precision%29) (Actor :type Symon%20Character%20Object%20Reference))
  ;[1 1 1] Comment
  (bind _output_get (Variables|Default|SetHealth (- (Variables|Default|GetHealth) Quantity)))
  (if (<= _output_get 0.0)
    (Physics|SetSimulatePhysics (Variables|Character|GetMesh) true)
    (Utilities|FlowControl|Delay 5.0)
    (Actor|DestroyActor (stale EventBeginPlay _returnvalue))
    (Actor|DestroyActor)
    (else
      (Utilities|IsValid Actor
        (:Is%20Valid
          (AI|AIMoveTo self (Transformation|GetActorLocation Actor) 0 8e+01 true))))))

(event Custom|ExecuteWayPath
  (bind _waypoints (Variables|Default|GetWayPoints))
  ;[1 1 1] Comment
  (if (not (== (Utilities|Array|Length (Variables|Default|GetWayPoints)) 0))
    (AI|AIMoveTo self "0, 0, 0" (Utilities|Array|Get(acopy) _waypoints (Variables|Default|GetCurrentWayPoint)) 1e+02 true
      (:OnSuccess
        (if (>= (Variables|Default|GetCurrentWayPoint) (- (Utilities|Array|Length _waypoints) 1))
          (Variables|Default|SetCurrentWayPoint 0)
          (else
            (Variables|Default|SetCurrentWayPoint (+ (Variables|Default|GetCurrentWayPoint) 1))))
        (Utilities|FlowControl|Delay (Variables|Default|GetDelay)))
      (:OnFail
        _))
    (CallFunction|ExecuteWayPath)))

(event EventBeginPlay
  (bind _self self)
  ;[1 1 1] Comment
  (CallFunction|ExecuteWayPath)
  (bind _returnvalue (Game|SpawnActorfromClass "/Game/ProjetoTCC/Blueprints/Weapons/EspadaBP.EspadaBP_C" (Math|Transform|MakeTransform "0, 0, 0") "Undefined" _self 0))
  (Transformation|AttachComponentToComponent _returnvalue (Variables|Character|GetMesh _self) "WeaponSocket" "KeepRelative" "KeepRelative" "KeepRelative" true))

(event EventIsAttackingBl
  (params (IsAttackingVar :type Boolean))
  ;[1 1 1] Comment
  (Variables|/Game/ProjetoTCC/Blueprints/Weapons/WeaponItem.WeaponItem_C|SetIsAttacking (stale EventBeginPlay _returnvalue) IsAttackingVar))

(event EventAllowAttackBl
  (params (AllowAttack :type Boolean))
  ;[1 1 1] Comment
  (Variables|Default|SetAllowAttacking AllowAttack))

(fn ConstructionScript)