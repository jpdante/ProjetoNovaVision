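; EspadaFoda is a sword weapon Blueprint that deals melee damage on contact.
; When the Espada component overlaps a CharacterBase other than its owner while IsAttacking is set, it applies fixed damage and spawns blood particles at Scene1.
; An AlreadyDamaged flag with a short delayed reset blocks repeat hits, so only one target takes damage per cooldown window.
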(event OnComponentBeginOverlap(espada)
  (params (OverlappedComponent :type Primitive%20Component%20Object%20Reference) (OtherActor :type Actor%20Object%20Reference) (OtherComp :type Primitive%20Component%20Object%20Reference) (OtherBodyIndex :type Integer) (bFromSweep :type Boolean) (SweepResult :type Hit%20Result%20Structure%20%28by%20ref%29))
  (if (not (Variables|Default|GetAlreadyDamaged))
    (if (not (== OtherActor (Components|GetOwner)))
      (if (Variables|Default|GetIsAttacking)
        (bind _ascharacter_base (Utilities|Casting|CastToCharacterBase OtherActor))
        (Default|TakeDamage _ascharacter_base 6e+01)
        (Effects|SpawnEmitteratLocation "/Game/ProjetoTCC/Particles/BloodParticles.BloodParticles" (Transformation|GetWorldLocation (Variables|Default|GetScene1)) "0, 0, 0" "2.000000,2.000000,2.000000")
        (Variables|Default|SetAlreadyDamaged true)
        (Utilities|FlowControl|Delay 0.6)
        (Variables|Default|SetAlreadyDamaged false)))))

(event EventBeginPlay)

(event Collision|EventActorBeginOverlap
  (params (OtherActor :type Actor%20Object%20Reference)))

(event EventTick
  (params (DeltaSeconds :type Float%20%28single-precision%29)))

(fn ConstructionScript)