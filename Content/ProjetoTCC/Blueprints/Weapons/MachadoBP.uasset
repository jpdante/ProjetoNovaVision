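; MachadoBP is an axe weapon that damages enemies its box collider overlaps while it is attacking.
; Overlapped Enemy1_Bp or Enemy_Strong actors go to CheckEnemy, which reduces health by a fixed amount and spawns a blood splatter emitter.
; The emitter's particle collisions are bound to ParticleCollide, which spawns short-lived, randomly sized blood decals using a dynamic material with a random frame.
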(event OnComponentBeginOverlap(Box)
  (params (OverlappedComponent :type Primitive%20Component%20Object%20Reference) (OtherActor :type Actor%20Object%20Reference) (OtherComp :type Primitive%20Component%20Object%20Reference) (OtherBodyIndex :type Integer) (bFromSweep :type Boolean) (SweepResult :type Hit%20Result%20Structure%20%28by%20ref%29))
  (if (Variables|Default|GetIsAttacking)
    (Utilities|FlowControl|Sequence
      (:then_0
        (bind _asenemy_1_bp (Utilities|Casting|CastToEnemy1_Bp OtherActor))
        (CallFunction|CheckEnemy (delegate Custom|ParticleCollide) _asenemy_1_bp))
      (:then_1
        (bind _asenemy_strong (Utilities|Casting|CastToEnemy_Strong OtherActor))
        (CallFunction|CheckEnemy (delegate Custom|ParticleCollide) _asenemy_strong)))))

(event Custom|ParticleCollide
  (params (EventName :type Name) (EmitterTime :type Float%20%28single-precision%29) (ParticleTime :type Integer) (Location :type Vector) (Velocity :type Vector) (Direction :type Vector) (Normal :type Vector) (BoneName :type Name) (PhysMat :type Physical%20Material%20Object%20Reference))
  (bind _returnvalue (Math|Random|RandomFloatinRange 2e+01 5e+01))
  (bind _returnvalue_2 (Rendering|Material|CreateDynamicMaterialInstance "/Game/ProjetoTCC/Particles/BloodDecal_Mat.BloodDecal_Mat" :!class /Script/Engine.KismetMaterialLibrary))
  (Rendering|Material|SetScalarParameterValue _returnvalue_2 "Frame" (Math|Conversions|ToFloat(Integer) (Math|Random|RandomInteger 11)) :!class /Script/Engine.MaterialInstanceDynamic)
  (Rendering|Decal|SpawnDecalatLocation _returnvalue_2 (Math|Vector|MakeVector 2.0 _returnvalue _returnvalue) Location "-90.000000,0.000000,0.000000" 2.0))

(event EventBeginPlay)

(event Collision|EventActorBeginOverlap
  (params (OtherActor :type Actor%20Object%20Reference)))

(event EventTick
  (params (DeltaSeconds :type Float%20%28single-precision%29)))

(fn ConstructionScript)

(fn CheckEnemy
  (params (Delegate :type %20Object%20Reference%20%28by%20ref%29) (Enemy :type Enemy%20Base%20Object%20Reference))
  (Default|ReduceHealth Enemy 3e+01)
  (bind _returnvalue (Effects|SpawnEmitteratLocation "/Game/ProjetoTCC/Particles/Splatter_P.Splatter_P" (Transformation|GetWorldLocation (Variables|Default|GetScene1)) "0, 0, 0" "0.400000,0.400000,0.400000"))
  (EventDispatchers|BindEventtoOnParticleCollide _returnvalue Delegate))