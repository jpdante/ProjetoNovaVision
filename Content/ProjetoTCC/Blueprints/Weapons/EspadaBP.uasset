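; EspadaBP is a sword weapon Blueprint, currently only printing the name of whatever overlaps its collision.
; A disconnected chain would, while attacking, damage SymonCharacter and spawn a blood splatter emitter bound to ParticleCollide.
; ParticleCollide spawns short-lived, randomly sized blood decals at impact points, using a dynamic material instance to pick a random frame.
; Since that binding never runs, both damage and blood effects are inactive.
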(event OnComponentBeginOverlap(Collision)
  (params (OverlappedComponent :type Primitive%20Component%20Object%20Reference) (OtherActor :type Actor%20Object%20Reference) (OtherComp :type Primitive%20Component%20Object%20Reference) (OtherBodyIndex :type Integer) (bFromSweep :type Boolean) (SweepResult :type Hit%20Result%20Structure%20%28by%20ref%29))
  (Development|PrintString (Utilities|GetObjectName OtherActor)))

(event Custom|ParticleCollide
  (params (EventName :type Name) (EmitterTime :type Float%20%28single-precision%29) (ParticleTime :type Integer) (Location :type Vector) (Velocity :type Vector) (Direction :type Vector) (Normal :type Vector) (BoneName :type Name) (PhysMat :type Physical%20Material%20Object%20Reference))
  (bind _returnvalue (Math|Random|RandomFloatinRange 2e+01 5e+01))
  (bind _returnvalue_2 (Rendering|Material|CreateDynamicMaterialInstance "/Game/ProjetoTCC/Particles/BloodDecal_Mat.BloodDecal_Mat" :!class /Script/Engine.KismetMaterialLibrary))
  (Rendering|Material|SetScalarParameterValue _returnvalue_2 "Frame" (Math|Conversions|ToFloat(Integer) (Math|Random|RandomInteger 11)) :!class /Script/Engine.MaterialInstanceDynamic)
  (Rendering|Decal|SpawnDecalatLocation _returnvalue_2 (Math|Vector|MakeVector 2.0 _returnvalue _returnvalue) Location "-90.000000,0.000000,0.000000" 2.0))

(event EventBeginPlay)

(event Collision|EventActorBeginOverlap
  (params (OtherActor :type Actor%20Object%20Reference)))

(event EventTick
  (params (DeltaSeconds :type Float%20%28single-precision%29)))

(fn ConstructionScript)