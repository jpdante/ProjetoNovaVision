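; BaseItem is a base item actor for world items such as herbs, wood, ores, coins, keys, fragments and boosts, defined by an ItemType and a Quantity.
; Its construction script clamps Quantity to at least one, then switches on ItemType to set the ItemMesh static mesh.
; Several types share a mesh, with a simple cube standing in for non-resource items.
; The event graph holds no active logic.
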(event EventBeginPlay)

(event Collision|EventActorBeginOverlap
  (params (OtherActor :type Actor%20Object%20Reference)))

(event EventTick
  (params (DeltaSeconds :type Float%20%28single-precision%29)))

(fn ConstructionScript
  (bind _itemmesh (Variables|Default|GetItemMesh))
  (if (< (Variables|Default|GetQuantity) 1)
    (Variables|Default|SetQuantity 1))
  (switch Utilities|FlowControl|Switch|SwitchonItems (Variables|Default|GetItemType)
    (:NewEnumerator0
      (Components|StaticMesh|SetStaticMesh _itemmesh "/Game/SoulCave/Environment/Meshes/Nature/SM_Cave_Grass01.SM_Cave_Grass01"))
    (:NewEnumerator1
      (Components|StaticMesh|SetStaticMesh _itemmesh "/Game/SoulCave/Environment/Meshes/Nature/SM_Cave_Grass01.SM_Cave_Grass01"))
    (:NewEnumerator2
      (Components|StaticMesh|SetStaticMesh _itemmesh "/Game/SoulCave/Environment/Meshes/Building/SM_Cave_Wood_Beam.SM_Cave_Wood_Beam"))
    (:NewEnumerator3
      (Components|StaticMesh|SetStaticMesh _itemmesh "/Game/ForestSet/Meshes/SM_Rock04.SM_Rock04"))
    (:NewEnumerator4
      (Components|StaticMesh|SetStaticMesh _itemmesh "/Game/ForestSet/Meshes/SM_Rock04.SM_Rock04"))
    (:NewEnumerator5
      (Components|StaticMesh|SetStaticMesh _itemmesh "/Game/ForestSet/Meshes/SM_Rock04.SM_Rock04"))
    (:NewEnumerator6
      (Components|StaticMesh|SetStaticMesh _itemmesh "/Game/Geometry/Meshes/1M_Cube.1M_Cube"))
    (:NewEnumerator7
      (Components|StaticMesh|SetStaticMesh _itemmesh "/Game/Geometry/Meshes/1M_Cube.1M_Cube"))
    (:NewEnumerator8
      (Components|StaticMesh|SetStaticMesh _itemmesh "/Game/Geometry/Meshes/1M_Cube.1M_Cube"))
    (:NewEnumerator9
      (Components|StaticMesh|SetStaticMesh _itemmesh "/Game/Geometry/Meshes/1M_Cube.1M_Cube"))))