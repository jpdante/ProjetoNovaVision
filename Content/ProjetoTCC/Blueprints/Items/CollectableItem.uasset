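; CollectableItem is a world pickup that the SymonCharacter collects with the F key when nearby.
; Sphere overlap tracks proximity and sets or clears the character's ActionableActorReference.
; Releasing F in range passes ItemType to the character's AddItem and destroys the actor.
; The construction script clamps Quantity to at least one, replaces empty or locked types with ErvaFraca, and picks the mesh per type, adding particles for keys.
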(event OnComponentBeginOverlap(Sphere)
  (params (OverlappedComponent :type Primitive%20Component%20Object%20Reference) (OtherActor :type Actor%20Object%20Reference) (OtherComp :type Primitive%20Component%20Object%20Reference) (OtherBodyIndex :type Integer) (bFromSweep :type Boolean) (SweepResult :type Hit%20Result%20Structure%20%28by%20ref%29))
  (bind _assymon_character (Utilities|Casting|CastToSymonCharacter OtherActor))
  (Variables|Default|SetSymonCharacter _assymon_character)
  (Variables|/Game/ProjetoTCC/Characters/Main/SymonCharacter.SymonCharacter_C|SetActionableActorReference _assymon_character self)
  (Variables|Default|SetPlayerIsClose true))

(event OnComponentEndOverlap(Sphere)
  (params (OverlappedComponent :type Primitive%20Component%20Object%20Reference) (OtherActor :type Actor%20Object%20Reference) (OtherComp :type Primitive%20Component%20Object%20Reference) (OtherBodyIndex :type Integer))
  (bind _assymon_character (Utilities|Casting|CastToSymonCharacter OtherActor))
  (Variables|Default|SetSymonCharacter 0)
  (Variables|/Game/ProjetoTCC/Characters/Main/SymonCharacter.SymonCharacter_C|SetActionableActorReference _assymon_character 0)
  (Variables|Default|SetPlayerIsClose false))

(event EventBeginPlay)

(event Collision|EventActorBeginOverlap
  (params (OtherActor :type Actor%20Object%20Reference)))

(event EventTick
  (params (DeltaSeconds :type Float%20%28single-precision%29)))

(event EventFReleased
  (if (Variables|Default|GetPlayerIsClose)
    (if true
      (Default|AddItem (Variables|Default|GetSymonCharacter) (Variables|Default|GetItemType))
      (Actor|DestroyActor))))

(fn ConstructionScript
  (bind _itemmesh (Variables|Components|GetItemMesh))
  (if (< (Variables|Default|GetQuantity) 1)
    (Variables|Default|SetQuantity 1))
  (switch Utilities|FlowControl|Switch|SwitchonCollectables (Variables|Default|GetItemType)
    (:NewEnumerator11
      (Variables|Default|SetItemType "NewEnumerator0"))
    (:NewEnumerator10
      (Variables|Default|SetItemType "NewEnumerator0"))
    (:NewEnumerator0
      (Components|StaticMesh|SetStaticMesh _itemmesh "/Game/ProjetoTCC/Blueprints/Items/Mesh/Erva1.Erva1"))
    (:NewEnumerator17
      (Components|StaticMesh|SetStaticMesh _itemmesh "/Game/SoulCave/Environment/Meshes/Nature/SM_Cave_Grass01.SM_Cave_Grass01"))
    (:NewEnumerator2
      (Components|StaticMesh|SetStaticMesh _itemmesh "/Game/InfinityBladeGrassLands/Environments/Misc/Exo_Deco01/StaticMesh/SM_WoodenBarrel_Destroyed.SM_WoodenBarrel_Destroyed"))
    (:NewEnumerator3
      (Components|StaticMesh|SetStaticMesh _itemmesh "/Game/ProjetoTCC/Blueprints/Items/Mesh/ferro.ferro")
      (Rendering|Material|SetMaterial (Variables|Components|GetItemMesh) 0 "/Game/GTFreeMaterials/Materials/Metal_BrushedCopper.Metal_BrushedCopper"))
    (:NewEnumerator4
      (Components|StaticMesh|SetStaticMesh _itemmesh "/Game/ProjetoTCC/Blueprints/Items/Mesh/ferro.ferro"))
    (:NewEnumerator5
      (Components|StaticMesh|SetStaticMesh _itemmesh "/Game/ProjetoTCC/Blueprints/Items/Mesh/ferro.ferro"))
    (:NewEnumerator6
      (Components|StaticMesh|SetStaticMesh _itemmesh "/Game/Geometry/Meshes/1M_Cube.1M_Cube"))
    (:NewEnumerator7
      (Components|StaticMesh|SetStaticMesh _itemmesh "/Game/ProjetoTCC/Blueprints/Items/Mesh/chave.chave" :!label _label)
      (AddComponent|AddParticleSystemComponent false (Math|Transform|MakeTransform "0.000000,10.000000,50.000000" "0, 0,-90.000000" "0.500000,0.500000,0.500000")))
    (:NewEnumerator18
      (goto _label))
    (:NewEnumerator19
      (goto _label))
    (:NewEnumerator8
      (Components|StaticMesh|SetStaticMesh _itemmesh "/Game/Geometry/Meshes/1M_Cube.1M_Cube"))
    (:NewEnumerator9
      (Components|StaticMesh|SetStaticMesh _itemmesh "/Game/Geometry/Meshes/1M_Cube.1M_Cube"))))